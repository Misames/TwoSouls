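; Melee Vanguard enemy Blueprint that handles taking damage and dying.
; AffectHealth subtracts damage from HealthPoint and triggers Death at zero or below.
; Death runs two timelines that animate the Amount parameter on dynamic materials for the body mesh and sword, creating a dissolve effect.
; A one-second Delay on the sword timeline's update then notifies the game mode of one fewer enemy and destroys the actor.
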(event Custom|Death
  ;[1 1 1] Death Handler
  (Utilities|FlowControl|Sequence
    (:then_0
      (bind _returnvalue (Rendering|Material|CreateDynamicMaterialInstance (Variables|Character|GetMesh) 1 0 "None" :!class /Script/Engine.PrimitiveComponent))
      (bind _amount (Timeline|Dissolution Play)
        (:Update
          (Rendering|Material|SetScalarParameterValue _returnvalue "Amount" _amount :!class /Script/Engine.MaterialInstanceDynamic)
          (Utilities|FlowControl|Delay 1.0))))
    (:then_1
      (bind _returnvalue_2 (Rendering|Material|CreateDynamicMaterialInstance (Variables|Default|GetSword_low-poly) 0 0 "None" :!class /Script/Engine.PrimitiveComponent))
      (bind _amount_2 (Timeline|Timeline_0 Play)
        (:Update
          (Rendering|Material|SetScalarParameterValue _returnvalue_2 "Amount" _amount_2 :!class /Script/Engine.MaterialInstanceDynamic)
          (Utilities|FlowControl|Delay 1.0)
          (Class|Activate|RemoveOneEnemy(Message) (Game|GetGameMode))
          (Actor|DestroyActor))))))

(event EventAffectHealth
  (params (Damage :type Integer))
  ;[1 1 1] Damage Handler
  (bind _output_get (Variables|Default|SetHealthPoint (- (Variables|Default|GetHealthPoint) Damage)))
  (if (<= _output_get 0)
    (CallFunction|Death)))

(fn ConstructionScript)