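; AI controller for enemy NPCs that starts the NPC_BT behavior tree on begin play and feeds it perception of the player.
; Each AIPerception update sets the PlayerInSight blackboard flag, true only when a Player-tagged actor is successfully sensed.
; On such a detection it also stores the player actor and location, which are not cleared when sensing fails.
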(event OnTargetPerceptionUpdated(AIPerception)
  (params (Actor :type Actor%20Object%20Reference) (Stimulus :type AI%20Stimulus%20Structure))
  (bind _bsuccessfullysensed (Utilities|Struct|BreakAIStimulus Stimulus))
  (bind _returnvalue (Actor|ActorHasTag Actor "Player"))
  (bind _self self)
  (bind _returnvalue_2 (AI|GetBlackboard _self))
  (bind _returnvalue_3 (and _returnvalue _bsuccessfullysensed))
  (AI|Components|Blackboard|SetValueasBool _returnvalue_2 (Utilities|Name|MakeLiteralName "PlayerInSight") _returnvalue_3)
  (if _returnvalue_3
    (AI|Components|Blackboard|SetValueasObject _returnvalue_2 (Utilities|Name|MakeLiteralName "PLayerActor") Actor)
    (AI|Components|Blackboard|SetValueasVector _returnvalue_2 (Utilities|Name|MakeLiteralName "PlayerLocation") (Transformation|GetActorLocation Actor))))

(event EventBeginPlay
  (AI|RunBehaviorTree "/Game/Blueprints/EnemyIA/NPC_BT.NPC_BT"))

(fn ConstructionScript)