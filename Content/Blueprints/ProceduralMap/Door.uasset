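; Door actor for a procedurally generated level that toggles open and closed on activation and builds the room behind it on first opening.
; Line traces measure free space: a hit on a door or wall yields a hall, otherwise side traces limit the new room's size and shift.
; A seeded random stream drives sizes, door counts and child room seeds, and doors drop to zero when GM_level1's room count reaches its maximum.
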(event Custom|NewRoom
  (params (Room%20Tiles%20X :type Integer) (Room%20Tiles%20Y :type Integer) (Shift :type Integer) (Max%20Doors :type Integer) (Hall :type Boolean))
  ;[1 1 1] Création nouvelle salle derière la porte
  (bind _asgm_level_1 (Utilities|Casting|CastToGM_level1 (Game|GetGameMode)))
  (Variables|/Game/Blueprints/ProceduralMap/GM_level1.GM_level1_C|SetNbRoomActual _asgm_level_1 (+ (Variables|/Game/Blueprints/ProceduralMap/GM_level1.GM_level1_C|GetNbRoomActual _asgm_level_1) 1))
  (Utilities|IsBossRoom?
    (:output
      (Game|SpawnActorfromClass "/Game/Blueprints/ProceduralMap/Room.Room_C" (Math|Transform|MakeTransform (+ (Transformation|GetActorLocation) (* (Transformation|GetActorForwardVector) 4e+02) "") (Math|Rotator|CombineRotators (Transformation|GetActorRotation) "0,90.000000, 0")) "Undefined" 0 Room%20Tiles%20X Room%20Tiles%20Y 4e+02 4e+02 (Variables|Default|GetNbDoors) Shift Hall (Class|KismetMathLibrary|RandomIntegerfromStream 10000 (Variables|Default|GetDoorStream)) 0))))

(event Custom|AddAddition
  (bind _returnvalue (Transformation|GetActorTransform))
  (bind _returnvalue_2 (Transformation|GetActorForwardVector))
  (bind _roomsizelimit (Variables|Default|GetroomSizeLimit))
  (bind _tilesize (Variables|Default|GettileSize))
  (bind _returnvalue_3 (Math|Transform|TransformLocation _returnvalue "200.000000,10.000000,200.000000"))
  (bind _returnvalue_4 (- _roomsizelimit 1))
  (bind _returnvalue_5 (* _returnvalue_4 _tilesize))
  (bind _returnvalue_6 (+ _returnvalue_5 1e+01))
  (bind _returnvalue_7 (* _returnvalue_2 _returnvalue_6))
  (bind (_outhit _returnvalue_8) (Collision|LineTraceByChannel _returnvalue_3 (+ _returnvalue_3 (* (Transformation|GetActorRightVector) (* (Variables|Default|GetroomSizeLimit) (Variables|Default|GettileSize)))) "TraceTypeQuery1" false 0 "None"))
  (if _returnvalue_8
    (switch string (Utilities|GetClassDisplayName (Utilities|GetClass (.HitActor (Collision|BreakHitResult _outhit))))
      (:Door
        (Utilities|Casting|CastToDoor (.HitActor (Collision|BreakHitResult _outhit)))
        (Variables|Default|Setroomify false))
      (:Wall%20collision
        (bind _aswall_collision (Utilities|Casting|CastTowallCollision (.HitActor (Collision|BreakHitResult _outhit))))
        (Default|RemoveIndex _aswall_collision)))
    (CallFunction|NewRoom (- (Math|Float|Round (/ (.Distance (Collision|BreakHitResult _outhit)) (Variables|Default|GettileSize))) 1) 1 0 (Variables|Default|GetNbDoors) true)
    (else
      (for _index (range 1 (- (Variables|Default|GetroomSizeLimit) 1))
        ;[1 1 1] limite gauche
        (Utilities|FlowControl|Sequence
          (:then_0
            (bind (_outhit_2 _returnvalue_9) (Collision|LineTraceByChannel (Math|Transform|TransformLocation (Transformation|GetActorTransform) (+ "390.000000,200.000000,300.000000" (Math|Vector|MakeVector 0.0 (* _index 4e+02) 0.0))) (+ (Math|Transform|TransformLocation (Transformation|GetActorTransform) (+ "390.000000,200.000000,300.000000" (Math|Vector|MakeVector 0.0 (* _index 4e+02) 0.0))) _returnvalue_7) "TraceTypeQuery1" false 0 "None"))
            (if _returnvalue_9
              (Variables|Default|SetLeftLimit (Math|Integer|Min(Integer) (Math|Float|Round (/ (.Distance (Collision|BreakHitResult _outhit_2)) (Variables|Default|GettileSize))) (Variables|Default|GetLeftLimit)))))
          (:then_1
            ;[1 1 1] limite droite
            (bind (_outhit_3 _returnvalue_10) (Collision|LineTraceByChannel (Math|Transform|TransformLocation (Transformation|GetActorTransform) (+ "10.000000,200.000000,300.000000" (Math|Vector|MakeVector 0.0 (* _index 4e+02) 0.0))) (+ (Math|Transform|TransformLocation (Transformation|GetActorTransform) (+ "10.000000,200.000000,300.000000" (Math|Vector|MakeVector 0.0 (* _index 4e+02) 0.0))) (* _returnvalue_7 -1.0)) "TraceTypeQuery1" false 0 "None"))
            (if _returnvalue_10
              (Variables|Default|SetRightLimit (Math|Integer|Min(Integer) (Math|Float|Round (/ (.Distance (Collision|BreakHitResult _outhit_3)) (Variables|Default|GettileSize))) (Variables|Default|GetRightLimit)))))))
      (Variables|Default|SetShift (Math|Random|RandomIntegerinRangefromStream 0 (Math|Integer|Min(Integer) (- (Variables|Default|GetroomSizeLimit) (Variables|Default|GetRightLimit)) (Variables|Default|GetLeftLimit)) (Variables|Default|GetDoorStream)))
      (CallFunction|NewRoom (Math|Random|RandomIntegerinRangefromStream 3 (Variables|Default|GetroomSizeLimit) (Variables|Default|GetDoorStream)) (+ (Variables|Default|GetRightLimit) (Variables|Default|GetShift) 1) (Variables|Default|GetShift) (Math|Random|RandomIntegerinRangefromStream 0 5 (Variables|Default|GetDoorStream)) false))))

(event Custom|Serv%20DoorStream
  (CallFunction|MultiDoorstream))

(event Custom|Multi%20Doorstream
  (Variables|Default|SetDoorStream (Math|Random|MakeRandomStream (Variables|Default|Getseed))))

(event EventBeginPlay
  (CallFunction|ServDoorStream))

(event EventActivated
  ;[1 1 1] Ouverture porte
  (if (Variables|Default|GetClosed)
    (Variables|Default|SetClosed false)
    (Utilities|FlowControl|Sequence
      (:then_0
        ;[1 1 1] La premiere fois qu'on ouvre une porte
        (if (Variables|Default|Getroomify)
          (Variables|Default|Setroomify false)
          (bind _output_get (Variables|Default|SetroomSizeLimit (Math|Random|RandomIntegerinRangefromStream 3 8 (Variables|Default|GetDoorStream))))
          (bind _output_get_2 (Variables|Default|SetLeftLimit _output_get))
          (Variables|Default|SetRightLimit _output_get_2)
          (CallFunction|AddAddition)))
      (:then_1
        (bind _newtrack_0 (Timeline|OpenDoorTimeline Play)
          (:Update
            (Transformation|SetRelativeRotation (Variables|Default|GetScene) (Math|Rotator|MakeRotator 0.0 0.0 _newtrack_0) false false)))))
    (else
      (Variables|Default|SetClosed true)
      (Timeline|OpenDoorTimeline Reverse))))

(fn ConstructionScript)

(fn OnRepClosed)

(fn OnRepRoomify)

(fn CanSpawnOneEnemy
  (return false))

(fn GetEnemyCount
  (return 0))