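; Procedural map room actor that builds itself on BeginPlay from a seeded stream, then reports to the game mode.
; It lays instanced floor tiles and edges them with seeded Door actors or instanced walls paired with WallCollision actors; halls skip end walls.
; Line traces avoid duplicating existing edges and clear Roomify on doors hit.
; RemoveWall swap-removes walls to keep indices aligned, and ActiveSpawner spawns melee enemies inside the spawner box.
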(event Custom|RemoveWall
  (params (index :type Integer))
  (bind _wall_collision (Variables|Default|GetWall%20collision))
  (bind _returnvalue (Utilities|Array|LastIndex _wall_collision))
  (bind _output (Utilities|Array|Get(acopy) _wall_collision _returnvalue))
  ;[1 1 1] supprimer le mur a l'index passé en parametre
  (Class|InstancedStaticMeshComponent|RemoveInstance (Variables|Default|Getwall2) index)
  (Utilities|Array|SetArrayElem _wall_collision index _output true)
  (Default|Update _output index)
  (Utilities|Array|RemoveIndex (Variables|Default|GetWall%20collision) _returnvalue))

(event Custom|Active%20Spawner
  (bind _spawner (Variables|Default|GetSpawner))
  (bind _asgm_level_1 (Utilities|Casting|CastToGM_level1 (Game|GetGameMode)))
  (for _index (range 1 (Variables|/Game/Blueprints/ProceduralMap/GM_level1.GM_level1_C|GetMaxEnemyCount _asgm_level_1))
    (AI|SpawnAIFromClass "/Game/Blueprints/EnemyIA/Enemy_Vanguard_Melee.Enemy_Vanguard_Melee_C" "/Game/Blueprints/EnemyIA/NPC_BT.NPC_BT" (Math|Random|RandomPointinBoundingBox (Transformation|GetWorldLocation _spawner) (Components|Box|GetScaledBoxExtent _spawner)) "0, 0, 0" true 0)
    (Class|Activate|AddOneEnemy(Message) (Game|GetGameMode))))

(event EventBeginPlay
  (Variables|Default|SetStream%20count (Math|Random|MakeRandomStream (Variables|Default|Getseed)))
  (CallFunction|UnderConstructionRoom)
  (Class|Activate|Spawner(Message) (Game|GetGameMode) self))

(fn ConstructionScript)

(fn UnderConstructionRoom
  (bind _roomtilesx (Variables|Default|GetRoomTilesX))
  (bind _roomtilesy (Variables|Default|GetRoomTilesY))
  (bind _returnvalue (- _roomtilesx 1))
  (bind _returnvalue_2 (- _roomtilesy 1))
  ;[1 1 1] Créer sol
  (for _index (range 0 _returnvalue_2)
    (for _index_2 (range 0 _returnvalue)
      (Components|InstancedStaticMesh|AddInstance (Variables|Components|Getfloor) (Math|Conversions|ToTransform(Vector) (Math|Vector|MakeVector (* (Variables|Default|GetTilesSizeX) (Math|Conversions|ToFloat(Integer) _index_2)) (* (Variables|Default|GetTilesSizeY) (Math|Conversions|ToFloat(Integer) (- _index (Variables|Default|GetEntry%20Shift)))) 0.0)))
      (if (== _index _returnvalue_2)
        (if (== _index_2 _returnvalue)
          (bind _output_get (Variables|Default|SetSpawner (Variables|Default|GetSpawner)))
          (Transformation|SetRelativeLocation _output_get (+ (.Location (Math|Transform|BreakTransform (Math|Conversions|ToTransform(Vector) (Math|Vector|MakeVector (* (Variables|Default|GetTilesSizeX) (Math|Conversions|ToFloat(Integer) _index_2)) (* (Variables|Default|GetTilesSizeY) (Math|Conversions|ToFloat(Integer) (- _index (Variables|Default|GetEntry%20Shift)))) 0.0)))) "0, 0,40.000000") false false)))))
  (if (not (Variables|Default|GetHall))
    (for _index_3 (range 0 (- (Variables|Default|GetRoomTilesY) 1))
      (if (or (Variables|Default|GetOrigin) (!= _index_3 (Variables|Default|GetEntry%20Shift)))
        ;[1 1 1] Mur du bas
        (CallFunction|WallorDoorReconstruction (== (Math|Integer|%(Integer) _index_3 (Variables|Default|GetDoor%20every%20%25)) (Variables|Default|Getdoor%20reminder)) (- (Math|Vector|MakeVector 0.0 (* (Variables|Default|GetTilesSizeY) (Math|Conversions|ToFloat(Integer) _index_3)) 0.0) (Math|Vector|MakeVector 0.0 (* (Variables|Default|GetEntry%20Shift) (Variables|Default|GetTilesSizeY)) 0.0)) "0,90.000000, 0"))
      ;[1 1 1] Mur du haut
      (CallFunction|WallorDoorReconstruction (== (Math|Integer|%(Integer) _index_3 (Variables|Default|GetDoor%20every%20%25)) (Variables|Default|Getdoor%20reminder)) (- (Math|Vector|MakeVector (* (Math|Conversions|ToFloat(Integer) (Variables|Default|GetRoomTilesX)) (Variables|Default|GetTilesSizeX)) (* (Variables|Default|GetTilesSizeY) (+ (Math|Conversions|ToFloat(Integer) _index_3) 1.0)) 0.0) (Math|Vector|MakeVector 0.0 (* (Variables|Default|GetEntry%20Shift) (Variables|Default|GetTilesSizeY)) 0.0)) "0,-90.000000, 0")))
  (for _index_4 (range 0 (- (Variables|Default|GetRoomTilesX) 1))
    ;[1 1 1] mur de droite
    (CallFunction|WallorDoorReconstruction (== (Math|Integer|%(Integer) _index_4 (Variables|Default|GetDoor%20every%20%25)) (Variables|Default|Getdoor%20reminder)) (- (Math|Vector|MakeVector (* (Variables|Default|GetTilesSizeX) (Math|Conversions|ToFloat(Integer) _index_4)) (* (Variables|Default|GetTilesSizeY) (Math|Conversions|ToFloat(Integer) (Variables|Default|GetRoomTilesY))) 0.0) (Math|Vector|MakeVector 0.0 (* (Variables|Default|GetEntry%20Shift) (Variables|Default|GetTilesSizeY)) 0.0)) "0, 0, 0")
    ;[1 1 1] Mur de gauche
    (CallFunction|WallorDoorReconstruction (== (Math|Integer|%(Integer) _index_4 (Variables|Default|GetDoor%20every%20%25)) (Variables|Default|Getdoor%20reminder)) (- (Math|Vector|MakeVector (* (Variables|Default|GetTilesSizeX) (+ (Math|Conversions|ToFloat(Integer) _index_4) 1.0)) 0.0 0.0) (Math|Vector|MakeVector 0.0 (* (Variables|Default|GetEntry%20Shift) (Variables|Default|GetTilesSizeY)) 0.0)) "0,180.000000, 0")))

(fn WallorDoorReconstruction
  (params (Can%20door%20? :type Boolean) (Transform%20location :type Vector) (Transform%20rotation :type Rotator))
  (bind _returnvalue (Transformation|GetActorTransform))
  (bind _doorcount (Variables|Default|GetDoorCount))
  (bind _returnvalue_2 (Math|Transform|TransformLocation _returnvalue Transform%20location))
  (bind _returnvalue_3 (Math|Transform|TransformRotation _returnvalue Transform%20rotation))
  (bind _returnvalue_4 (Math|Transform|MakeTransform _returnvalue_2 _returnvalue_3))
  (Utilities|CheckWall Transform%20location Transform%20rotation
    (:false
      (if (and Can%20door%20? (Class|KismetMathLibrary|RandomBoolwithWeightfromStream (/ (Math|Conversions|ToFloat(Integer) (- _doorcount (Utilities|Array|Length (Variables|Default|GetDoor)))) (Math|Conversions|ToFloat(Integer) _doorcount)) (Variables|Default|GetStream%20count)))
        ;[1 1 1] Si on peut faire spawn une door on spawn une door
        (bind _returnvalue_5 (Game|SpawnActorfromClass "/Game/Blueprints/ProceduralMap/Door.Door_C" _returnvalue_4 "Undefined" 0 (Class|KismetMathLibrary|RandomIntegerfromStream 10000 (Variables|Default|GetStream%20count)) 0))
        (Utilities|Array|Add (Variables|Default|GetDoor) _returnvalue_5)
        (else
          ;[1 1 1] sinon un mur
          (bind _returnvalue_6 (Components|InstancedStaticMesh|AddInstance (Variables|Default|Getwall2) (Math|Transform|MakeTransform Transform%20location Transform%20rotation)))
          (bind _returnvalue_7 (Game|SpawnActorfromClass "/Game/Blueprints/ProceduralMap/wallCollision.wallCollision_C" _returnvalue_4 "Undefined" 0 _returnvalue_6 self 0))
          (Utilities|Array|AddUnique (Variables|Default|GetWall%20collision) _returnvalue_7))))))

(fn OnRepStreamCount)

(fn OnRepDoor)