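; Game mode for the procedural level 1, managing two-player spawning, enemy count and room opening state.
; When two players are present, the first tracked controller possesses a spawned BP_Player and the other a BP_Compagnon.
; Tick sets CanOpen false only while enemies remain and the room count differs from its maximum.
; Enemy add/remove events feed a spawn-cap check; session-based kick and spawn logic is present but never runs.
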(event EventOnLogout
  (params (ExitingController :type Controller%20Object%20Reference))
  (bind _asplayer_controller (Utilities|Casting|CastToPlayerController ExitingController))
  (Utilities|Array|RemoveItem (Variables|Default|GetPlayer%20Controllers) _asplayer_controller))

(event EventTick
  (params (DeltaSeconds :type Float%20%28single-precision%29))
  (if (and (!= (Variables|Default|GetNbRoomActual) (Variables|Default|GetNbRoomMax)) (!= (Variables|Default|GetCurrentEnemyCount) 0))
    (Variables|Default|SetCanOpen false)
    (else
      (Variables|Default|SetCanOpen true))))

(event EventHandleStartingNewPlayer
  (params (NewPlayer :type Player%20Controller%20Object%20Reference))
  (Utilities|Array|AddUnique (Variables|Default|GetPlayer%20Controllers) NewPlayer)
  (if (== (Utilities|Array|Length (Variables|/Script/Engine.GameStateBase|GetPlayerArray (Game|GetGameState))) 2)
    (for (_array_element _array_index) (Variables|Default|GetPlayer%20Controllers)
      (if (== _array_index 0)
        (bind _returnvalue (Game|SpawnActorfromClass "/Game/Blueprints/Player/BP_Player.BP_Player_C" (Math|Transform|MakeTransform "60.000000,60.000000,60.000000" "0, 0, 0" "1,1,1") "AdjustIfPossibleButAlwaysSpawn" 0 0))
        (Pawn|Possess _array_element _returnvalue)
        (else
          (bind _returnvalue_2 (Game|SpawnActorfromClass "/Game/Blueprints/Player/BP_Compagnon.BP_Compagnon_C" (Math|Transform|MakeTransform "100.000000,100.000000,100.000000" "0, 0, 0" "1,1,1") "Undefined" 0 0))
          (Pawn|Possess _array_element _returnvalue_2))))))

(event EventSpawner
  (params (RoomSpawner :type Room%20Object%20Reference))
  (Variables|Default|SetRoomSpawner RoomSpawner)
  (Utilities|Time|SetTimerbyEvent (EventDispatchers|CreateEvent (Variables|Default|GetRoomSpawner) :!event ActiveSpawner) 0.1))

(event EventAddOneEnemy
  ;[1 1 1] Gère le nombre d'ennemi présent dans le level
  (Math|Integer|IncrementInt (Variables|Default|GetCurrentEnemyCount)))

(event EventRemoveOneEnemy
  ;[1 1 1] Gère le nombre d'ennemi présent dans le level
  (Math|Integer|DecrementInt (Variables|Default|GetCurrentEnemyCount)))

(fn ConstructionScript)

(fn CanSpawnOneEnemy
  (return (< (Variables|Default|GetCurrentEnemyCount) (Variables|Default|GetMaxEnemyCount))))

(fn GetEnemyCount
  (return (Variables|Default|GetCurrentEnemyCount)))