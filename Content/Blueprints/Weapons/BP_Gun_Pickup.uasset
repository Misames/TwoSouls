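; Weapon pickup that gives a gun to the BP_Player or BP_Compagnon that overlaps its box.
; The overlap passes through ServGetWeapon to MultiGetWeapon, named as a server-to-multicast chain, so the spawn happens inside the multicast-named event.
; That event spawns ClassWeapon, sets it as the character's CurrentWeapon, attaches it to the mesh's socket_weapon and destroys the pickup.
; It does not handle any previously held weapon.
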(event OnComponentBeginOverlap(Box)
  (params (OverlappedComponent :type Primitive%20Component%20Object%20Reference) (OtherActor :type Actor%20Object%20Reference) (OtherComp :type Primitive%20Component%20Object%20Reference) (OtherBodyIndex :type Integer) (bFromSweep :type Boolean) (SweepResult :type Hit%20Result%20Structure%20%28by%20ref%29))
  (CallFunction|ServGetWeapon OtherActor))

(event Custom|Serv%20GetWeapon
  (params (Other%20Actor :type Object%20Object%20Reference))
  (CallFunction|MultiGetWeapon Other%20Actor))

(event Custom|Multi%20GetWeapon
  (params (Other%20Actor :type Object%20Object%20Reference))
  (if (== (Utilities|GetClass Other%20Actor) "/Game/Blueprints/Player/BP_Compagnon.BP_Compagnon_C")
    (bind _asbp_compagnon (Utilities|Casting|CastToBP_Compagnon Other%20Actor))
    (bind _returnvalue (Game|SpawnActorfromClass (Variables|Default|GetClassWeapon) (Math|Transform|MakeTransform "0, 0, 0" "0, 0, 0" "1,1,1") "Undefined" 0 0))
    (bind _output_get (Variables|/Game/Blueprints/Player/BP_Compagnon.BP_Compagnon_C|SetCurrentWeapon _asbp_compagnon _returnvalue))
    (Transformation|AttachComponentToComponent _output_get (Variables|/Script/Engine.Character|GetMesh _asbp_compagnon) "socket_weapon" "KeepRelative" "KeepRelative" "KeepRelative" true)
    (Actor|DestroyActor)
    (else
      (bind _asbp_player (Utilities|Casting|CastToBP_Player Other%20Actor))
      (bind _returnvalue_2 (Game|SpawnActorfromClass (Variables|Default|GetClassWeapon) (Math|Transform|MakeTransform "0, 0, 0" "0, 0, 0" "1,1,1") "Undefined" 0 0))
      (bind _output_get_2 (Variables|/Game/Blueprints/Player/BP_Player.BP_Player_C|SetCurrentWeapon _asbp_player _returnvalue_2))
      (Transformation|AttachComponentToComponent _output_get_2 (Variables|/Script/Engine.Character|GetMesh _asbp_player) "socket_weapon" "KeepRelative" "KeepRelative" "KeepRelative" true)
      (Actor|DestroyActor))))

(fn ConstructionScript)