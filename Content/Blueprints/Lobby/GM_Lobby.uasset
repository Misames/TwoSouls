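; Lobby game mode that gathers connecting players and starts the match once the session is full.
; PostLogin tracks controllers, waits on a retriggerable delay, then compares the player count to the session's connection limit, kicking extra players as "Serveur Complet".
; At or over the limit, it updates the LAN session, then server-travels to Level1 after a short delay.
; Logout removes the controller from the tracked list.
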(event EventBeginPlay)

(event EventTick
  (params (DeltaSeconds :type Float%20%28single-precision%29)))

(event EventPostLogin
  (params (NewPlayer :type Player%20Controller%20Object%20Reference))
  (Utilities|Array|AddUnique (Variables|Default|GetPlayerControllers) NewPlayer)
  (Utilities|FlowControl|RetriggerableDelay 2.0)
  ;[1 1 1] si on a trop de joueur
  (bind (_numconnections _numprivateconnections _bislan _bisdedicated _ballowinvites _ballowjoininprogress _bisanticheatenabled _builduniqueid _extrasettings) (Class|AdvancedSessionsLibrary|GetSessionSettings)
    (:OnSuccess
      (if (> (Utilities|Array|Length (Variables|/Script/Engine.GameStateBase|GetPlayerArray (Game|GetGameState))) _numconnections)
        ;[1 1 1] on les kick
        (bind (_arrayindex _arrayelement) (Utilities|Array|ReverseforEachLoop (Variables|Default|GetPlayerControllers))
          (:LoopBody
            (if (>= _arrayindex _numconnections)
              (Class|AdvancedSessionsLibrary|KickPlayer _arrayelement "Serveur Complet")))
          (:Completed
            (|UpdateSession _extrasettings _numconnections 0 true false false true false :!label _label
              (:OnSuccess
                (Utilities|FlowControl|Delay 3.0)
                (Development|ExecuteConsoleCommand "serverTravel Level1" 0)))))
        (elif (== (Utilities|Array|Length (Variables|/Script/Engine.GameStateBase|GetPlayerArray (Game|GetGameState))) _numconnections)
          (goto _label))))))

(event EventOnLogout
  (params (ExitingController :type Controller%20Object%20Reference))
  (bind _asplayer_controller (Utilities|Casting|CastToPlayerController ExitingController))
  (Utilities|Array|RemoveItem (Variables|Default|GetPlayerControllers) _asplayer_controller))

(fn ConstructionScript)